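; Projectile Blueprint that, on hit, spawns an explosion emitter and timed decal, then applies damage credited to a player controller.
; ShootBullet passes speed, effect scales and damage to SetupBullet, calls Fire, then stores the bullet type.
; Fire sets ProjectileMovement velocity along an arrow's forward vector and also applies it as a velocity-change impulse to the Bullet mesh.
; The bullet is not destroyed on hit, and bouncing only prints debug text.
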(event `self.ReceiveTick`
  (params (DeltaSeconds :type "Float (single-precision)")))

(event `self.bullet.OnComponentHit`
  (params (HitComponent :type "PrimitiveComponent Object Reference") (OtherActor :type "Actor Object Reference") (OtherComp :type "PrimitiveComponent Object Reference") (NormalImpulse :type "Vector Structure") (Hit :type "HitResult Structure (by ref)"))
  (bind (_bblockinghit _binitialoverlap _time _distance _location _impactpoint _normal _impactnormal _physmat _hitactor) (`GameplayStatics.BreakHitResult` Hit))
  (`self.PlayImpactEffect` _impactpoint _impactnormal)
  (`self.ApplyDamage` _hitactor (`self.Bullet Damge`)))

(event `self.ProjectileMovement.OnProjectileBounce`
  (params (ImpactResult :type "HitResult Structure (by ref)") (ImpactVelocity :type "Vector Structure (by ref)"))
  (`KismetSystemLibrary.PrintString` "Hello"))

(fn `ApplyDamage`
  (params (`HitActor ` :type "Actor Object Reference") (`DamageAmount ` :type "Float (double-precision)") (Player :type Integer))
  (`GameplayStatics.ApplyDamage` `HitActor ` `DamageAmount ` (`GameplayStatics.GetPlayerController` Player) self))

(fn `Fire`
  (params (ArrowComp :type "ArrowComponent Object Reference"))
  (bind _projectilemovement (`self.ProjectileMovement`))
  (bind _output_get (set `MovementComponent.Velocity` (* (`ProjectileMovementComponent.InitialSpeed` _projectilemovement) (`SceneComponent.GetForwardVector` ArrowComp)) _projectilemovement))
  (`PrimitiveComponent.AddImpulse` (`self.bullet`) _output_get "None" true))

(fn `PlayImpactEffect`
  (params (`ImpactLocation ` :type "Vector Structure") (`ImpactNormal ` :type "Vector Structure"))
  (bind _returnvalue (`KismetMathLibrary.Conv_VectorToRotator` `ImpactNormal `))
  (`GameplayStatics.SpawnEmitterAtLocation` "/Game/StarterContent/Particles/P_Explosion.P_Explosion" `ImpactLocation ` _returnvalue (`KismetMathLibrary.Conv_DoubleToVector` (`self.Emitter PFX Scale`)) true "AutoRelease")
  (`GameplayStatics.SpawnDecalAtLocation` "/Engine/EditorMaterials/Cascade/CASC_RenderLights_MAT.CASC_RenderLights_MAT" (`KismetMathLibrary.Conv_DoubleToVector` (`self.Impact FX Scale`)) `ImpactLocation ` _returnvalue 10.0))

(fn `SetupBullet`
  (params (`Arrow Comp In` :type "ArrowComponent Object Reference") (initialSpeed :type "Float (double-precision)") (maxSpeed :type "Float (double-precision)") (`Emitter Scale` :type "Float (double-precision)") (`Impact Scale` :type "Float (double-precision)") (`Bullet Damge` :type "Float (double-precision)"))
  (returns (`Arrow Comp Out` :type "ArrowComponent Object Reference"))
  (bind _projectilemovement (`self.ProjectileMovement`))
  (bind _bullet (`self.bullet`))
  (`StaticMeshComponent.SetStaticMesh` _bullet (`StaticMeshComponent.StaticMesh` _bullet))
  (set `ProjectileMovementComponent.InitialSpeed` initialSpeed _projectilemovement)
  (set `ProjectileMovementComponent.MaxSpeed` maxSpeed _projectilemovement)
  (set `self.Emitter PFX Scale` `Emitter Scale`)
  (set `self.Impact FX Scale` `Impact Scale`)
  (set `self.Bullet Damge` `Bullet Damge`)
  (return `Arrow Comp In`))

(fn `ShootBullet`
  (params (ArrowComp :type "ArrowComponent Object Reference") (Speed :type "Float (double-precision)" :default 30000.0) (`Emitter PFX Scale` :type "Float (double-precision)" :default 1.0) (`Impact FX Scale` :type "Float (double-precision)" :default 5.0) (`Bullet Damge` :type "Float (double-precision)" :default 500.0) (BulletType :type "/Game/BulletTypes Enum" :default "NewEnumerator0"))
  (bind _arrow_comp_out (`self.SetupBullet` ArrowComp Speed 100000.0 `Emitter PFX Scale` `Impact FX Scale` `Bullet Damge`))
  (`self.Fire` _arrow_comp_out)
  (set `self.BulletType` BulletType))

(fn `UserConstructionScript`)